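; BP_PhysicsMachine1 is a physics-driven machine actor that travels along world -Y according to how fast its Door component, acting as a rotor, spins.
; Each Tick subtracts the magnitude of the Door's angular velocity from the actor's Y, so either spin direction moves it the same way, without delta-time scaling.
; It then snaps the Door to a fixed Y offset from the actor, keeping the rotor attached as it moves.
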(event EventTick
  (params (DeltaSeconds :type Float%20%28single-precision%29))
  (bind _returnvalue (Transformation|GetActorLocation))
  (bind _returnvalue_2 (Transformation|GetActorLocation))
  (bind _door (Variables|Default|GetDoor))
  (bind (_x _y _z) (Math|Vector|BreakVector _returnvalue_2))
  (bind (_x_2 _y_2 _z_2) (Math|Vector|BreakVector _returnvalue))
  ;[0.15 0 0 0.5] Actor Movement
  (Transformation|SetActorLocation (Math|Vector|MakeVector _x_2 (+ (* (Math|Vector|VectorLength (Class|PrimitiveComponent|GetPhysicsAngularVelocityinRadians _door "None")) -1.0) _y_2) _z_2) false false)
  ;[0.15 0 0.003536 0.5] Rotor Movement
  (Transformation|SetWorldLocation _door (Math|Vector|MakeVector _x (+ _y 9e+01) _z) false false))

(fn ConstructionScript)