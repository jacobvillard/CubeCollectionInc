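; AI pawn with a cube mesh that chases the player and shows moods on a face widget.
; Pawn sensing sets chase blackboard keys and starts a looping line-trace check that clears HasSeenPlayer on any blocking hit.
; Player overlap shows love, while projectile hits or UpdateFace pick a negative mood, each drawing a random texture from its array.
; While Reenable is set, Tick disables mesh physics and snaps the actor to the mesh.
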(event OnSeePawn(PawnSensing)
  (params (Pawn :type Pawn%20Object%20Reference))
  (bind _self self)
  (bind _returnvalue (AI|GetAIController _self))
  (bind _returnvalue_2 (AI|GetBlackboard _returnvalue))
  (Utilities|Casting|CastToBP_FirstPersonCharacter Pawn)
  (AI|Components|Blackboard|SetValueasBool _returnvalue_2 (Utilities|Name|MakeLiteralName "HasSeenPlayer") true)
  (AI|Components|Blackboard|SetValueasBool _returnvalue_2 (Utilities|Name|MakeLiteralName "Chase") true)
  (Utilities|Time|ClearTimerbyFunctionName 0 "CheckLostSight")
  (Utilities|Time|SetTimerbyFunctionName 0 "CheckLostSight" 2.5 true))

(event OnComponentBeginOverlap(Box)
  (params (OverlappedComponent :type Primitive%20Component%20Object%20Reference) (OtherActor :type Actor%20Object%20Reference) (OtherComp :type Primitive%20Component%20Object%20Reference) (OtherBodyIndex :type Integer) (bFromSweep :type Boolean) (SweepResult :type Hit%20Result%20Structure%20%28by%20ref%29))
  (Utilities|Casting|CastToBP_FirstPersonCharacter OtherActor
    (:then
      (CallFunction|SetFaceState "love"))
    (:CastFailed
      (Utilities|Casting|CastToBP_FirstPersonProjectile OtherActor)
      (Development|PrintString "should work")
      (switch int (Math|Random|RandomInteger 4)
        (:0
          (CallFunction|SetFaceState "angry"))
        (:1
          (CallFunction|SetFaceState "trapped"))
        (:2
          (CallFunction|SetFaceState "scared"))
        (:3
          (CallFunction|SetFaceState "sad"))))))

(event Custom|UpdateFace
  (Development|PrintString "should work")
  (switch int (Math|Random|RandomInteger 4)
    (:0
      (CallFunction|SetFaceState "angry"))
    (:1
      (CallFunction|SetFaceState "trapped"))
    (:2
      (CallFunction|SetFaceState "scared"))
    (:3
      (CallFunction|SetFaceState "sad"))))

(event EventBeginPlay
  (CallFunction|SetFaceState "happy"))

(event EventTick
  (params (DeltaSeconds :type Float%20%28single-precision%29))
  (bind _cubemesh (Variables|Default|GetCubeMesh))
  (if (Variables|Default|GetReenable)
    (Physics|SetSimulatePhysics _cubemesh false)
    (Transformation|SetActorLocation (Transformation|GetWorldLocation _cubemesh) false false)))

(event EventEndPlay
  (params (EndPlayReason :type EEndPlayReason%20Enum :default "Destroyed"))
  (Development|PrintString (Utilities|String|EnumtoString EndPlayReason)))

(fn ConstructionScript)

(fn CheckLostSight
  (bind _outhit (Collision|LineTraceByChannel (Transformation|GetActorLocation) (Transformation|GetActorLocation (Game|GetPlayerCharacter 0)) "TraceTypeQuery1" false 0 "None"))
  (Development|PrintString (Utilities|String|ToString(Boolean) (.bBlockingHit (Collision|BreakHitResult _outhit))))
  (if (.bBlockingHit (Collision|BreakHitResult _outhit))
    (AI|Components|Blackboard|SetValueasBool (AI|GetBlackboard (AI|GetAIController self)) (Utilities|Name|MakeLiteralName "HasSeenPlayer") false)))

(fn SetFaceState
  (params (Mode :type String))
  (if (Utilities|Enum|Equal(Enum) Mode "happy")
    (CallFunction|SetFacePNG (Variables|Default|GetHappy))
    (elif (Utilities|Enum|Equal(Enum) Mode "shocked")
      (CallFunction|SetFacePNG (Variables|Default|GetShocked))
      (elif (Utilities|Enum|Equal(Enum) Mode "sad")
        (CallFunction|SetFacePNG (Variables|Default|GetSad))
        (elif (Utilities|Enum|Equal(Enum) Mode "scared")
          (CallFunction|SetFacePNG (Variables|Default|GetScared))
          (elif (Utilities|Enum|Equal(Enum) Mode "angry")
            (CallFunction|SetFacePNG (Variables|Default|GetAngry))
            (elif (Utilities|Enum|Equal(Enum) Mode "trapped")
              (CallFunction|SetFacePNG (Variables|Default|GetTrapped))
              (elif (Utilities|Enum|Equal(Enum) Mode "love")
                (CallFunction|SetFacePNG (Variables|Default|GetLove))
                (else
                  (Development|PrintString "Thats not a valid mood dumbass"))))))))))

(fn SetFacePNG
  (params (TexArray :type Array%20of%20Texture%202D%20Object%20References))
  (bind _asbp_cube_face (Utilities|Casting|CastToBP_CubeFace (UserInterface|GetUserWidgetObject (Variables|Default|GetWidget))))
  (Default|UpdateImage _asbp_cube_face (Utilities|Array|Get(acopy) TexArray (Math|Random|RandomIntegerinRange 0 (- (Utilities|Array|Length TexArray) 1)))))